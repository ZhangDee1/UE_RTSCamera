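; RTS demo player controller that shows the mouse cursor and handles hover and click interaction with world objects.
; A Tick trace under the cursor, throttled by a Delay, finds WorldDynamic actors implementing BPI_RTS_Interact.
; The hovered actor receives a hover message and supplies debug text to BP_RTS_HUD, which clears when nothing qualifies.
; Left click sends the interact message to the currently hovered actor.
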(event `self.ReceiveBeginPlay`
  (`|ExecutionSequence`
    (:`then_0`
      (set `self.bShowMouseCursor` true))
    (:`then_1`
      (`KismetSystemLibrary.Delay` 0.2)
      (bind _asbp_rts_hud (cast `/Game/RTSDemo/Blueprint/Gameplay/BP_RTS_HUD` (`self.GetHUD`)))
      (set `self.HUD` _asbp_rts_hud))))

(event `self.ReceiveTick`
  (params (DeltaSeconds :type "Float (single-precision)"))
  (bind (_hitresult _returnvalue) (`self.GetHitResultUnderCursorForObjects` (`|MakeArray` "ObjectTypeQuery2" :!type "EObjectTypeQuery Enum")))
  (bind (_bblockinghit _binitialoverlap _time _distance _location _impactpoint _normal _impactnormal _physmat _hitactor) (`GameplayStatics.BreakHitResult` _hitresult))
  (`KismetSystemLibrary.Delay` 0.1) ; 限制检测评率，另外这种检测方式也并不是很推荐，看下Cropout Sample,可以发现其实在主角下挂一个Collision，然后跟随鼠标位置做交互
  (if _returnvalue
    (if (`KismetSystemLibrary.DoesImplementInterface` _hitactor "/Game/RTSDemo/Interface/BPI_RTS_Interact.BPI_RTS_Interact_C")
      (bind _output_get (set `self.OnHoveredActor` _hitactor))
      (message `/Game/RTSDemo/Interface/BPI_RTS_Interact.OnMouseHover` _output_get)
      (bind _content (message `/Game/RTSDemo/Interface/BPI_RTS_Interact.GetDebugInfo` _output_get))
      (set `/Game/RTSDemo/Blueprint/Gameplay/BP_RTS_HUD.DisplayText` _content (`self.HUD`))
      (else
        (set `self.OnHoveredActor` null)
        (set `/Game/RTSDemo/Blueprint/Gameplay/BP_RTS_HUD.DisplayText` "" (`self.HUD`))))
    (else
      (set `self.OnHoveredActor` null)
      (set `/Game/RTSDemo/Blueprint/Gameplay/BP_RTS_HUD.DisplayText` "" (`self.HUD`)))))

(event `Key|LeftMouseButton`
  (params (Key :type "Key Structure"))
  (bind _onhoveredactor (`self.OnHoveredActor`))
  ;[1 1 1] 为了保持插件目录干净，所以鼠标左键放这里，
  (:`Pressed`
    (`/Engine/EditorBlueprintResources/StandardMacros.IsValid` _onhoveredactor
      (:`Is Valid`
        (message `/Game/RTSDemo/Interface/BPI_RTS_Interact.OnInteract` _onhoveredactor)))))

(fn `UserConstructionScript`)