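; BP_BuildingBase is a base interactable building for the RTS demo, providing hover highlighting, a click-style interaction and debug info.
; Its decal starts hidden, and each hover event shows it and restarts a short retriggerable delay that hides it again once hovering stops.
; Interaction, marked TODO, sets the RTS pawn's TargetVector to the building's location, and GetDebugInfo returns DisplayInfo.
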(event `self.ReceiveBeginPlay`
  (`SceneComponent.SetHiddenInGame` (`self.Decal`) true false))

(event `/Game/RTSDemo/Interface/BPI_RTS_Interact.OnMouseHover`
  (`SceneComponent.SetHiddenInGame` (`self.Decal`) false false)
  (`KismetSystemLibrary.RetriggerableDelay` 0.2)
  (`SceneComponent.SetHiddenInGame` (`self.Decal`) true false))

(event `/Game/RTSDemo/Interface/BPI_RTS_Interact.OnInteract`
  (bind _asbp_rts_pawn (cast `/RTSCamera/Core/BP_RTS_Pawn` (`GameplayStatics.GetPlayerPawn` 0)))
  (set `/RTSCamera/Core/BP_RTS_Pawn.TargetVector` (`self.K2_GetActorLocation`) _asbp_rts_pawn))

(fn `GetDebugInfo`
  (returns (Content :type String))
  (return (`self.DisplayInfo`)))

(fn `UserConstructionScript`)